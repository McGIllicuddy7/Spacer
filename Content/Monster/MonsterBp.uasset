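; Monster actor that moves toward the player's pawn using a NavNetBP actor from the level as its NavMesh.
; On BeginPlay it caches the first NavNetBP, waits briefly, then issues a single MoveTo to the pawn's location at that moment, with no re-targeting.
; When direct movement finishes, a callback optionally rotates it to face the move-to location.
; MoveTo and RotateTo are defined outside these graphs.
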(event `self.ReceiveBeginPlay`
  (bind _outactors (`GameplayStatics.GetAllActorsOfClass` "/Game/Framework/Navigation/NavNetBP.NavNetBP_C"))
  (set `self.NavMesh` (`|GetArrayItem` _outactors))
  (`KismetSystemLibrary.Delay` 0.2)
  (`self.MoveTo` (`self.K2_GetActorLocation` (`Controller.K2_GetPawn` (`GameplayStatics.GetPlayerController` 0)))))

(event `self.ReceiveTick`
  (params (DeltaSeconds :type "Float (single-precision)")))

(event `self.FinishedMovingDirectlyCallback`
  (if (`self.Should Rortate To Move To Location`)
    (bind _returnvalue (`self.GetMoveToLocation`))
    (`self.RotateTo` (`KismetMathLibrary.FindLookAtRotation` (`self.K2_GetActorLocation`) _returnvalue))))

(fn `UserConstructionScript`)