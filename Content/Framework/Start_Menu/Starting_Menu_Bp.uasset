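; Start menu Blueprint that handles loading a saved game, starting a new game and exiting.
; LoadSave reads the level name from the save game, sets a LoadedSave flag in a separate Load_Level_Info slot, creating it if missing, then opens that level.
; NewGame opens NewMap and writes a fresh save game recording that level name.
; Exit quits through a console command.
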(event `Load Save`
  (bind _save_game (`/Game/Framework/Save_Namss.Save Game Save Name`))
  (bind _load_level_save_name (`/Game/Framework/Save_Namss.Load Level Save Name`))
  (bind _returnvalue (`GameplayStatics.DoesSaveGameExist` _save_game))
  (if _returnvalue
    (bind _returnvalue_2 (`GameplayStatics.LoadGameFromSlot` _save_game))
    (bind _assave_game_info (cast `/Game/Framework/Save_Game_Info` _returnvalue_2))
    (bind _returnvalue_3 (`GameplayStatics.DoesSaveGameExist` _load_level_save_name))
    (if _returnvalue_3
      (bind _returnvalue_4 (`GameplayStatics.LoadGameFromSlot` _load_level_save_name))
      (bind _asload_level_info (cast `/Game/Framework/Load_Level_Info` _returnvalue_4))
      (set `/Game/Framework/Load_Level_Info.Loaded Save` true _asload_level_info)
      (`GameplayStatics.SaveGameToSlot` _asload_level_info _load_level_save_name)
      (else
        (bind _returnvalue_5 (`GameplayStatics.CreateSaveGameObject` "/Game/Framework/Load_Level_Info.Load_Level_Info_C"))
        (set `/Game/Framework/Load_Level_Info.Loaded Save` true _returnvalue_5)
        (`GameplayStatics.SaveGameToSlot` _returnvalue_5 _load_level_save_name)))
    (`GameplayStatics.OpenLevel` (`KismetStringLibrary.Conv_StringToName` (`/Game/Framework/Save_Game_Info.Level Name` _assave_game_info)))))

(event `New Game +`
  (`GameplayStatics.OpenLevel` "NewMap")
  (bind _returnvalue (`GameplayStatics.CreateSaveGameObject` "/Game/Framework/Save_Game_Info.Save_Game_Info_C"))
  (set `/Game/Framework/Save_Game_Info.Level Name` (`KismetStringLibrary.Conv_NameToString` "NewMap") _returnvalue)
  (`GameplayStatics.SaveGameToSlot` _returnvalue (`/Game/Framework/Save_Namss.Save Game Save Name`)))

(event `Exit`
  (`KismetSystemLibrary.ExecuteConsoleCommand` "exit" null))

(fn `UserConstructionScript`)