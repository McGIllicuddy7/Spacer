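; Navigation network actor that builds its net at BeginPlay from the NavNode_t actors placed in the level.
; Generate collects each node actor's location and hands the list to GenerateNet, which is defined outside this Blueprint.
; A disconnected debug graph can draw capsules at the resulting Nodes and lines to their index-based Neighbors, separating link directions by color and height.
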(event `self.ReceiveBeginPlay`
  (`self.Generate`))

(fn `Generate`
  (locals (Locations :type "Array of Vector Structure"))
  (bind _outactors (`GameplayStatics.GetAllActorsOfClass` "/Game/Framework/Navigation/NavNode_t.NavNode_t_C"))
  (for _array_element _outactors
    (`KismetArrayLibrary.Array_Add` (`local.Locations`) (`self.K2_GetActorLocation` _array_element)))
  (`self.GenerateNet` (`local.Locations`)))

(fn `UserConstructionScript`)